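; Spawner actor that places three interactable pickups in the level when play begins.
; On BeginPlay it spawns an InteractablePickupBP at each of its three spawn point components, using their world transforms and owning the spawned actors.
; The construction script randomizes the actor's yaw while keeping roll and pitch, so the layout of the spawn points rotates randomly around the spawner.
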(event EventBeginPlay
  (Game|SpawnActorfromClass "/Game/Blueprints/InteractablePickupBP.InteractablePickupBP_C" (Transformation|GetWorldTransform (Variables|Default|GetSpawnPoint1)) "Undefined" self 0)
  (Game|SpawnActorfromClass "/Game/Blueprints/InteractablePickupBP.InteractablePickupBP_C" (Transformation|GetWorldTransform (Variables|Default|GetSpawnPoint2)) "Undefined" self 0)
  (Game|SpawnActorfromClass "/Game/Blueprints/InteractablePickupBP.InteractablePickupBP_C" (Transformation|GetWorldTransform (Variables|Default|GetSpawnPoint3)) "Undefined" self 0))

(fn ConstructionScript
  (bind _returnvalue (Transformation|GetActorRotation))
  (bind (_roll _pitch) (Math|Rotator|BreakRotator _returnvalue))
  (Transformation|SetActorRotation (Math|Rotator|MakeRotator _roll _pitch (Math|Random|RandomFloatinRange 0.0 3.6e+02))))