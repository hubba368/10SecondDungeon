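; MapGenTestBP is a test dungeon map-generation actor that populates its section with walls, object spawners and flying enemies.
; BeginPlay spawns an offset LevelWalls_Blueprint at one-third of the actor's scale.
; BeginSpawning, once the game instance reports game start, places InteractableObjSpawners at five points and FlyingEnemyBPs above up to four others.
; The enemy loop runs inclusively to the max turret count, in fixed order; random-pick and list-removal nodes are unwired.
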(event Custom|BeginSpawning
  (bind _asdungeon_game_instance (Utilities|Casting|CastToDungeonGameInstance (Game|GetGameInstance)))
  (if (Variables|/Script/DreamMachine.DungeonGameInstance|GetHasGameStarted _asdungeon_game_instance)
    (Variables|Default|SetFlyingSpawnList (Utilities|Array|MakeArray (Variables|Default|GetFlyingSpawn) (Variables|Default|GetFlyingSpawn2) (Variables|Default|GetFlyingSpawn3) (Variables|Default|GetFlyingSpawn4)))
    (bind _output_get (Variables|Default|SetObjSpawnList (Utilities|Array|MakeArray (Variables|Default|GetObjSpawn1) (Variables|Default|GetObjSpawn2) (Variables|Default|GetObjSpawn3) (Variables|Default|GetObjSpawn4) (Variables|Default|GetObjSpawn5))))
    (for (_ _array_index) _output_get
      (Variables|Default|SetTempIndex _array_index)
      (Game|SpawnActorfromClass "/Game/Blueprints/InteractableObjSpawner.InteractableObjSpawner_C" (Math|Transform|MakeTransform (.Location (Math|Transform|BreakTransform (Transformation|GetWorldTransform (Utilities|Array|Get(acopy) _output_get _array_index)))) (.Rotation (Math|Transform|BreakTransform (Transformation|GetWorldTransform (Utilities|Array|Get(acopy) _output_get _array_index)))) (Math|Vector|MakeVector 1.0 1.0 1.0)) "Undefined" 0 0))
    (bind _asdungeon_game_instance_2 (Utilities|Casting|CastToDungeonGameInstance (Game|GetGameInstance)))
    (Variables|Default|SetFlyingCounter 0)
    (bind _returnvalue (Class|DungeonGameInstance|GetMaxTurretCount _asdungeon_game_instance_2))
    (while (<= (Variables|Default|GetFlyingCounter) _returnvalue)
      (AI|SpawnAIFromClass "/Game/Blueprints/FlyingEnemyBP.FlyingEnemyBP_C" 0 (+ (Transformation|GetWorldLocation (Utilities|Array|Get(acopy) (Variables|Default|GetFlyingSpawnList) (Variables|Default|GetFlyingCounter))) "0, 0,200.000000") "0, 0, 0" false)
      (Math|Integer|IncrementInt (Variables|Default|GetFlyingCounter)))))

(event EventBeginPlay
  (bind _self self)
  (bind _returnvalue (Transformation|GetActorTransform _self))
  (bind (_location _rotation _scale) (Math|Transform|BreakTransform _returnvalue))
  (bind (_x _y _z) (Math|Vector|BreakVector _scale))
  (bind (_x_2 _y_2 _z_2) (Math|Vector|BreakVector _location))
  (Game|SpawnActorfromClass "/Game/Blueprints/LevelWalls_Blueprint.LevelWalls_Blueprint_C" (Math|Transform|MakeTransform (Math|Vector|MakeVector _x_2 (+ _y_2 2.7e+02) _z_2) _rotation (Math|Vector|MakeVector (/ _x 3.0) (/ _y 3.0) (/ _z 3.0))) "Undefined" _self 0))

(fn ConstructionScript)