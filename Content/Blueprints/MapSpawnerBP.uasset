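; Map spawner actor that populates the dungeon with walker enemies when BeginSpawning is called, provided the game has started.
; It calls SpawnWalker until EnemyCounter exceeds the game instance's MaxEnemyCount, retrying failed attempts.
; Each walker spawns at a random nearby navmesh point and joins CurrentEnemyList, which the first spawn resets.
; The proximity check uses signed offsets and re-rolls the random point, so it never validates the actual spawn location.
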(event Custom|BeginSpawning
  (Variables|Default|SetEnemyCounter 0)
  (bind _asdungeon_game_instance (Utilities|Casting|CastToDungeonGameInstance (Game|GetGameInstance)))
  (if (Variables|/Script/DreamMachine.DungeonGameInstance|GetHasGameStarted _asdungeon_game_instance)
    (while (<= (Variables|Default|GetEnemyCounter) (Variables|/Script/DreamMachine.DungeonGameInstance|GetMaxEnemyCount _asdungeon_game_instance))
      (if (== (Variables|Default|GetEnemyCounter) 0)
        (CallFunction|SpawnWalker true)
        (else
          (CallFunction|SpawnWalker false (Variables|Default|GetEnemyCounter)))))))

(event EventBeginPlay)

(fn ConstructionScript)

(fn SpawnWalker
  (params (SpawnFirstActor :type Boolean) (CurrentEnemyIndex :type Integer))
  (bind _self self)
  (bind _returnvalue (Transformation|GetActorLocation _self))
  (bind _randomlocation (Class|NavigationSystem|GetRandomPointinNavigableRadius _returnvalue 1e+03))
  (bind _returnvalue_2 (- _returnvalue _randomlocation))
  (bind (_x _y _z) (Math|Vector|BreakVector _returnvalue_2))
  (bind _returnvalue_3 (< _x 1e+02))
  (bind _returnvalue_4 (< _y 1e+02))
  (bind _returnvalue_5 (< _z 1e+02))
  (bind _returnvalue_6 (Math|Boolean|ANDBoolean _returnvalue_3 _returnvalue_4 _returnvalue_5))
  (if SpawnFirstActor
    (if (not _returnvalue_6)
      (bind _returnvalue_7 (AI|SpawnAIFromClass "/Game/Blueprints/WalkerEnemyBP.WalkerEnemyBP_C" 0 _randomlocation "0, 0, 0" false))
      (bind _asdungeon_game_instance (Utilities|Casting|CastToDungeonGameInstance (Game|GetGameInstance)))
      (Variables|/Script/DreamMachine.DungeonGameInstance|SetCurrentEnemyList _asdungeon_game_instance (Utilities|Array|MakeArray _returnvalue_7))
      (Math|Integer|IncrementInt (Variables|Default|GetEnemyCounter)))
    (elif (not _returnvalue_6)
      (bind _returnvalue_8 (AI|SpawnAIFromClass "/Game/Blueprints/WalkerEnemyBP.WalkerEnemyBP_C" 0 _randomlocation "0, 0, 0" false))
      (bind _asdungeon_game_instance_2 (Utilities|Casting|CastToDungeonGameInstance (Game|GetGameInstance)))
      (Utilities|Array|Add (Variables|/Script/DreamMachine.DungeonGameInstance|GetCurrentEnemyList _asdungeon_game_instance_2) _returnvalue_8)
      (Math|Integer|IncrementInt (Variables|Default|GetEnemyCounter)))))