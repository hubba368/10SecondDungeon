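; StartGameTriggerBP is a one-shot trigger that starts the game's enemies by setting them to the IDLE state when overlapped.
; On begin overlap it finds every WalkerEnemyBP and FlyingEnemyBP in the level, calls SetNewState on each, then destroys itself.
; The PlayerCharacterBP check only gates a debug name print, so any overlapping actor fires the trigger.
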(event Collision|EventActorBeginOverlap
  (params (OtherActor :type Actor%20Object%20Reference))
  (if (== OtherActor "/Game/Player/PlayerCharacterBP.PlayerCharacterBP")
    (Development|PrintString (Utilities|GetDisplayName OtherActor)))
  (bind _outactors (Actor|GetAllActorsOfClass "/Game/Blueprints/WalkerEnemyBP.WalkerEnemyBP_C"))
  (for _array_element _outactors
    (Class|BaseEnemy|SetNewState _array_element "IDLE"))
  (bind _outactors_2 (Actor|GetAllActorsOfClass "/Game/Blueprints/FlyingEnemyBP.FlyingEnemyBP_C"))
  (for _array_element_2 _outactors_2
    (Class|BaseEnemy|SetNewState _array_element_2 "IDLE"))
  (Actor|DestroyActor))

(fn ConstructionScript)