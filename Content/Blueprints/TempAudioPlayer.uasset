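; TempAudioPlayer is a Blueprint that starts background music when a level begins.
; On BeginPlay it compares the current level name to MenuScene, assigns either MenuMusic or BattleMusic to its Audio component, and plays it from the start.
; Unconnected nodes hold an unused path for storing a music timestamp in DungeonGameInstance, so playback position is not carried between levels here.
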(event EventBeginPlay
  (bind _audio (Variables|Default|GetAudio))
  (bind _returnvalue (Game|GetCurrentLevelName true))
  (if (Utilities|Enum|Equal(Enum) _returnvalue "MenuScene")
    (Audio|Components|Audio|SetSound _audio "/Game/Audio/MenuMusic.MenuMusic")
    (Audio|Components|Audio|Play _audio 0.0)
    (else
      (Audio|Components|Audio|SetSound _audio "/Game/Audio/BattleMusic.BattleMusic")
      (Audio|Components|Audio|Play _audio 0.0))))

(event EventTick
  (params (DeltaSeconds :type Float%20%28single-precision%29)))

(fn ConstructionScript)