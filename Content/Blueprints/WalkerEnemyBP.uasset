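; WalkerEnemyBP is a walker enemy that hurts the player on contact and recoils from hits.
; A capsule hit on the player character applies damage, then switches to the ABILITY state, halts AI movement and launches the walker backwards by setting its velocity.
; Taking any damage alternates between two hit sounds via FlipFlop, then runs the same state change and recoil.
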(event OnComponentHit(CapsuleComponent)
  (params (HitComponent :type Primitive%20Component%20Object%20Reference) (OtherActor :type Actor%20Object%20Reference) (OtherComp :type Primitive%20Component%20Object%20Reference) (NormalImpulse :type Vector :default "0, 0, 0") (Hit :type Hit%20Result%20Structure%20%28by%20ref%29))
  (bind _returnvalue (Game|GetPlayerCharacter 0))
  (bind _self self)
  (bind _returnvalue_2 (AI|GetAIController _self))
  (if (!= OtherActor 0)
    (if (!= OtherActor "WalkerEnemyBP")
      (if (!= OtherComp 0)
        (if (== OtherActor _returnvalue)
          (Game|Damage|ApplyDamage _returnvalue 1.0 _returnvalue_2 _self)
          (Class|BaseEnemy|SetNewState _self "ABILITY")
          (AI|Navigation|StopMovement _returnvalue_2)
          (Variables|/Script/Engine.MovementComponent|SetVelocity (Variables|Character|GetCharacterMovement) (* (Math|Vector|NegateVector (Math|Rotator|GetRotationXVector (Transformation|GetActorRotation _self))) 3.5e+03)))))))

(event Game|Damage|EventAnyDamage
  (params (Damage :type Float%20%28single-precision%29) (DamageType :type Damage%20Type%20Object%20Reference) (InstigatedBy :type Controller%20Object%20Reference) (DamageCauser :type Actor%20Object%20Reference))
  (bind _self self)
  (bind _audio (Variables|Default|GetAudio))
  (Utilities|FlowControl|FlipFlop
    (:A
      (Audio|Components|Audio|SetSound _audio "/Game/Audio/WalkerHit1.WalkerHit1"))
    (:B
      (Audio|Components|Audio|SetSound _audio "/Game/Audio/GhostHit2.GhostHit2")))
  (Audio|Components|Audio|AdjustVolume _audio 0.0 1.5e+02 :!class /Script/Engine.AudioComponent)
  (Audio|Components|Audio|Play _audio 0.0)
  (Class|BaseEnemy|SetNewState _self "ABILITY")
  (AI|Navigation|StopMovement (AI|GetAIController _self))
  (Variables|/Script/Engine.MovementComponent|SetVelocity (Variables|Character|GetCharacterMovement) (* (Math|Vector|NegateVector (Math|Rotator|GetRotationXVector (Transformation|GetActorRotation _self))) 3.5e+03)))

(fn ConstructionScript)