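; Player character Blueprint that plays an attack sound when flagged.
; Tick polls the PlayAttackAudio flag and, through a DoOnce that resets immediately, sets the Audio component's volume, plays it from the start and clears the flag.
; A separate test function returns Height times Width plus Width, apparently an experiment in grid index math, and is not called here.
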(event EventTick
  (params (DeltaSeconds :type Float%20%28single-precision%29))
  (bind _audio (Variables|Default|GetAudio))
  (if (Variables|Default|GetPlayAttackAudio)
    (Utilities|FlowControl|DoOnce false :!label _label
      (:Completed
        (Audio|Components|Audio|AdjustVolume _audio 0.0 25.0 :!class /Script/Engine.AudioComponent)
        (Audio|Components|Audio|Play _audio 0.0)
        (Variables|Default|SetPlayAttackAudio false)
        (goto _label Reset)))))

(fn ConstructionScript)

(fn Testgetindexfunction
  (params (width :type Integer) (height :type Integer))
  (return (+ (* height width) width)))